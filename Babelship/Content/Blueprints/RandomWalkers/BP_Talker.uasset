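; BP_Talker is a random-walker Blueprint that can display talking text through a widget component.
; On BeginPlay it sets the widget's visibility from IsSpeaking and passes its TalkingText to the Widget_Talker instance.
; Every tick it turns the widget to face the player character on yaw only, keeping pitch and roll at zero.
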(event EventBeginPlay
  (bind _widget (Variables|Default|GetWidget))
  (Rendering|SetVisibility _widget (Variables|Default|GetIsSpeaking) false)
  (bind _aswidget_talker (Utilities|Casting|CastToWidget_Talker (UserInterface|GetWidget _widget)))
  (Variables|/Game/Blueprints/RandomWalkers/Widget_Talker.Widget_Talker_C|SetTalkingText _aswidget_talker (Variables|Default|GetTalkingText)))

(event EventTick
  (params (DeltaSeconds :type Float%20%28single-precision%29))
  (Transformation|SetWorldRotation (Variables|Default|GetWidget) (Math|Rotator|MakeRotator 0.0 0.0 (+ (.yaw (Math|Rotator|FindLookatRotation (Transformation|GetActorLocation (Game|GetPlayerCharacter 0)) (Transformation|GetActorLocation self))) 1.8e+02)) false false))

(fn ConstructionScript)